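; Paper2D side-scrolling player character with running, double and wall jumps, velocity-based dash launch, climbing and a timed projectile attack.
; Tick flips the sprite by X velocity and picks its flipbook through a priority-ordered state function.
; Climbing uses Flying movement with input-driven play rate while CanClimb is set, and wall jumps use a line trace to launch away from walls.
; Jumping and landing spawn dust and drive timeline squash-and-stretch on actor scale.
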(event Custom|Wall%20Jump
  (bind _returnvalue (Transformation|GetActorLocation))
  (bind _returnvalue_2 (Transformation|GetActorForwardVector))
  (bind _capsulecomponent (Variables|Collision|GetCapsuleComponent))
  (bind _returnvalue_3 (Components|Capsule|GetScaledCapsuleRadius _capsulecomponent))
  (bind _returnvalue_4 (+ _returnvalue_3 15.0))
  ;[1 1 1] Wall Jump
  (bind (_outhit _returnvalue_5) (Collision|LineTraceByChannel (- _returnvalue (* _returnvalue_2 _returnvalue_4)) (+ _returnvalue (* _returnvalue_2 _returnvalue_4)) "TraceTypeQuery1" true 0 "None"))
  (if _returnvalue_5
    (Character|LaunchCharacter (Math|Vector|MakeVector (* (Math|Float|Sign(Float) (- (.x (Transformation|GetActorLocation)) (.x (.Location (Collision|BreakHitResult _outhit))))) 4.5e+02) 0.0 (Variables|/Script/Engine.CharacterMovementComponent|GetJumpZVelocity (Variables|Character|GetCharacterMovement))) false false)))

(event Custom|UpdateAnimation
  ;[1 1 1] Animation Event Control
  (Variables|Default|SetbIsMoving (Math|Vector|NotEqual(Vector) (Transformation|GetVelocity) "0, 0,0.000000" 0.0001))
  (bind _outputfb (CallFunction|AnimationStateMachine (Variables|Default|GetbIsMoving) (AI|Components|NavMovement|IsFalling (Variables|Character|GetCharacterMovement)) (Variables|Default|GetbIsAttacking) (Variables|Default|GetbIsDashing) (Variables|Default|GetbIsClimbing)))
  (Sprite|SetFlipbook (Variables|Default|GetSprite) _outputfb))

(event Custom|Fire%20Projectile
  ;[1 1 1] Attack
  (Game|SpawnActorfromClass "/Game/Blueprints/ProjectileBP.ProjectileBP_C" (Transformation|GetWorldTransform (Variables|Default|GetProjectileSpawn)) "Undefined" 0 0))

(event Custom|AttackAnimation
  ;[1 1 1] Attack
  (Utilities|FlowControl|Sequence
    (:then_0
      (Variables|Default|SetbIsAttacking true)
      (Utilities|FlowControl|Delay 0.2)
      (CallFunction|FireProjectile))
    (:then_1
      (Utilities|FlowControl|Delay 0.3)
      (Variables|Default|SetbIsAttacking false))))

(event Custom|LandFX
  ;[1 1 1] Jump Effects
  (Effects|SpawnEmitteratLocation "/Game/Art/Particles/pDust.pDust" (Transformation|GetWorldLocation (Variables|Default|GetDustBox)))
  (bind _squash (Timeline|Timeline_1 PlayFromStart)
    (:Update
      (Transformation|SetActorScale3D (Math|Vector|Lerp(Vector) "1.000000,1.000000,1.000000" "2.500000,1.000000,0.200000" _squash)))))

(event Custom|ClimbingEnd
  ;[1 1 1] Climbing
  (if (Variables|Default|GetbIsClimbing)
    (Pawn|Components|CharacterMovement|SetMovementMode (Variables|Character|GetCharacterMovement) "MOVE_Walking" 0)
    (Variables|Default|SetbIsClimbing false)
    (Components|Timeline|SetPlayRate (Variables|Default|GetSprite) 1.0)))

(event Custom|JumpFX
  ;[1 1 1] Jump Effects
  (Effects|SpawnEmitteratLocation "/Game/Art/Particles/pDust.pDust" (Transformation|GetWorldLocation (Variables|Default|GetDustBox)))
  (bind _squash (Timeline|Timeline_0 PlayFromStart)
    (:Update
      (Transformation|SetActorScale3D (Math|Vector|Lerp(Vector) "1.000000,1.000000,1.000000" "0.200000,1.000000,2.500000" _squash)))))

(event EventTick
  (params (DeltaSeconds :type Float%20%28single-precision%29))
  ;[1 1 1] Update
  (CallFunction|UpdateAnimation)
  (Math|Float|CompareFloat (.X (Math|Vector|BreakVector (Variables|/Script/Engine.MovementComponent|GetVelocity (Variables|Character|GetCharacterMovement)))) 0.0
    (:>
      (Transformation|SetRelativeRotation (Variables|Default|GetSprite) "0, 0, 0" false false))
    (:<
      (Transformation|SetRelativeRotation (Variables|Default|GetSprite) "0,180.000000, 0" false false))))

(event EventOnLanded
  (params (Hit :type Hit%20Result%20Structure%20%28by%20ref%29))
  ;[1 1 1] Landed
  (CallFunction|LandFX))

(event Input|ActionEvents|InputActionJump
  (params (Key :type Key%20Structure))
  ;[1 1 1] Jumping
  (:Pressed
    (if (Class|NavMovementComponent|IsFlying (Variables|Character|GetCharacterMovement))
      (Character|LaunchCharacter "0, 0,400.000000" false false)
      (CallFunction|ClimbingEnd)
      (else
        (Character|Jump)
        (if (AI|Components|NavMovement|IsFalling (Variables|Character|GetCharacterMovement))
          (CallFunction|WallJump))
        (CallFunction|JumpFX))))
  (:Released
    (Character|StopJumping)))

(event Input|ActionEvents|InputActionAttack
  (params (Key :type Key%20Structure))
  ;[1 1 1] Attack
  (:Pressed
    (if (not (Variables|Default|GetbIsAttacking))
      (CallFunction|AttackAnimation))))

(event Input|ActionEvents|InputActionDash
  (params (Key :type Key%20Structure))
  (bind _returnvalue (Transformation|GetVelocity))
  ;[1 1 1] Dash
  (:Pressed
    (if (Math|Vector|NotEqual(Vector) _returnvalue "0, 0, 0" 0.0001)
      (Character|LaunchCharacter (* (+ _returnvalue "0, 0, 0") "1.500000,1.500000,1.500000") false false))))

(event Input|AxisEvents|InputAxisMoveUp
  (params (AxisValue :type Float%20%28single-precision%29))
  ;[1 1 1] Climbing
  (if (Variables|Default|GetbCanClimb)
    (if (Math|Float|InRange(Float) AxisValue -0.1 0.1)
      (if (Class|NavMovementComponent|IsFlying (Variables|Character|GetCharacterMovement))
        (Components|Timeline|SetPlayRate (Variables|Default|GetSprite) 0.0))
      (else
        (Variables|Default|SetbIsClimbing true)
        (Components|Timeline|SetPlayRate (Variables|Default|GetSprite) AxisValue)
        (Pawn|Components|CharacterMovement|SetMovementMode (Variables|Character|GetCharacterMovement) "MOVE_Flying" 0)
        (Pawn|Input|AddMovementInput "0, 0,0.500000" AxisValue false)))))

(event Input|AxisEvents|InputAxisMoveRight
  (params (AxisValue :type Float%20%28single-precision%29))
  ;[1 1 1] Movement Control
  (Pawn|Input|AddMovementInput "1.000000, 0, 0" AxisValue false))

(fn ConstructionScript
  (Variables|/Script/Engine.CharacterMovementComponent|SetJumpZVelocity (Variables|Character|GetCharacterMovement) 4e+02)
  (Variables|Default|SetJumpMaxHoldTime 0.3)
  (Variables|Default|SetJumpMaxCount 2))

(fn AnimationStateMachine
  (params (bIsMoving :type Boolean) (bIsFalling :type Boolean) (bIsAttacking :type Boolean) (bIsDashing :type Boolean) (bIsClimbing :type Boolean))
  (if bIsClimbing
    (LocalVariables|SetAnimationState "NewEnumerator5")
    (elif bIsDashing
      (LocalVariables|SetAnimationState "NewEnumerator3")
      (elif bIsAttacking
        (LocalVariables|SetAnimationState "NewEnumerator4")
        (elif bIsFalling
          (LocalVariables|SetAnimationState "NewEnumerator2")
          (elif bIsMoving
            (LocalVariables|SetAnimationState "NewEnumerator1")
            (else
              (LocalVariables|SetAnimationState "NewEnumerator0")))))))
  (return (Utilities|Select :Index (LocalVariables|GetAnimationState) :NewEnumerator0 "/Game/Art/Sprite/Nephalem/idle/fNephalemIdle.fNephalemIdle" :NewEnumerator1 "/Game/Art/Sprite/Nephalem/walking/fNephalemWalking.fNephalemWalking" :NewEnumerator2 "/Game/Art/Sprite/Nephalem/jump/fNephalemJump.fNephalemJump" :NewEnumerator3 "/Game/Art/Sprite/Nephalem/dash/fNephalemDashBlock.fNephalemDashBlock" :NewEnumerator4 "/Game/Art/Sprite/Nephalem/attacking/fNephalemAttack2.fNephalemAttack2" :NewEnumerator5 "/Game/Art/Sprite/Nephalem/climbing/fClimbing.fClimbing")))