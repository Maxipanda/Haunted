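; Ladder actor that builds its rungs and box volume procedurally from the LadderBottom and LadderTop points.
; The construction script stacks squashed Paper2D sprites without collision every RungOffset units along the vertical distance between those points.
; It then scales the Box component by half that height and raises it by the same amount to span the ladder.
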(fn ConstructionScript
  (bind _rungoffset (Variables|Default|GetRungOffset))
  (bind _box (Variables|Default|GetBox))
  (bind _laddertop (Variables|Default|GetLadderTop))
  (bind _ladderbottom (Variables|Default|GetLadderBottom))
  (bind _returnvalue (- _laddertop _ladderbottom))
  (bind _returnvalue_2 (/ (.z _returnvalue) 2.0))
  (for _index (range 0 (Math|Float|Truncate (/ (.z _returnvalue) _rungoffset)))
    (bind _returnvalue_3 (AddComponent|AddPaperSpriteComponent false (Math|Transform|MakeTransform (Math|Vector|MakeVector 0.0 0.0 (* _index _rungoffset)) "0, 0, 0" "1,1,0.100000")))
    (Rendering|Components|Sprite|SetSprite _returnvalue_3 (Variables|Default|GetLadderSprite))
    (Collision|SetCollisionEnabled _returnvalue_3 "NoCollision"))
  (Transformation|SetRelativeScale3D _box (Math|Vector|MakeVector 1.0 1.0 _returnvalue_2))
  (Transformation|AddRelativeLocation _box (Math|Vector|MakeVector 0.0 0.0 _returnvalue_2) false false))