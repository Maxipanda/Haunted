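; Bomb actor that its 0_Base owner charges, releases on attack, and that explodes through the owner's BombExplosion once charge time exceeds the maximum.
; Server-authority Tick accumulates charge, even after launch, and launches when the owner is Attacking; AttackCheck always passes.
; LaunchBomb detaches the bomb, stores the aim direction and clears SpecialAction.
; Aim-offset and charge-scaling updates are never run, and launched movement is left unwired.
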(event Custom|BombExplode
  (Default|BombExplosion (.As0%20Base (Utilities|Casting|CastTo0_Base (Variables|Default|GetTheOwner))) self)
  (Actor|DestroyActor))

(event Custom|LaunchBomb
  (bind _theowner (Variables|Default|GetTheOwner))
  (bind _as0_base (Utilities|Casting|CastTo0_Base _theowner))
  (Variables|Default|SetbombLaunched? true)
  (Transformation|DetachFromActor "KeepWorld" "KeepWorld" "KeepWorld")
  (Transformation|SetActorLocation (+ (* (Variables|/Game/Blueprints/Character/0_Base.0_Base_C|GetAimingDirection (.As0%20Base (Utilities|Casting|CastTo0_Base (Variables|Default|GetTheOwner)))) 3e+01) (Math|Vector|MakeVector 0.0 0.0 1.0)) false false)
  (Variables|/Game/Blueprints/Character/0_Base.0_Base_C|SetspecialAction? _as0_base false)
  (Variables|Default|SetlaunchDirection (Variables|/Game/Blueprints/Character/0_Base.0_Base_C|GetAimingDirection _as0_base)))

(event Custom|updateBombPosition
  (if (Variables|Default|GetbombLaunched?)
    (Development|PrintString (Utilities|String|ToString(Vector) (Transformation|GetWorldLocation (Variables|Default|GetDefaultSceneRoot))))
    (else
      (Transformation|SetActorRelativeTransform (Math|Transform|MakeTransform (+ (* (Variables|/Game/Blueprints/Character/0_Base.0_Base_C|GetAimingDirection (.As0%20Base (Utilities|Casting|CastTo0_Base (Variables|Default|GetTheOwner)))) 3e+01) (Math|Vector|MakeVector 0.0 0.0 1.0)) "0, 0, 0" (Math|Conversions|ToVector(Float) (Variables|Default|GetCurrentChargeTime))) false false))))

(event EventTick
  (params (DeltaSeconds :type Float%20%28single-precision%29))
  (Networking|SwitchHasAuthority
    (:Authority
      (Variables|Default|SetDeltaTime DeltaSeconds)
      (bind _output_get (Variables|Default|SetCurrentChargeTime (+ DeltaSeconds (Variables|Default|GetCurrentChargeTime))))
      (if (> _output_get (Variables|Default|GetChargeTimeMax))
        (CallFunction|BombExplode)
        (elif (not (Variables|Default|GetbombLaunched?))
          (if (Variables|/Game/Blueprints/Character/0_Base.0_Base_C|Getattacking? (.As0%20Base (Utilities|Casting|CastTo0_Base (Variables|Default|GetTheOwner))))
            (bind _hit_ (CallFunction|AttackCheck))
            (if _hit_
              (CallFunction|LaunchBomb))))))))

(fn ConstructionScript
  (Variables|Default|SetBombSpeed 1e+02))

(fn AttackCheck
  (return true))