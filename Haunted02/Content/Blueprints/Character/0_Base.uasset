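; Base 2D knight character with eight-direction movement, a timed dash and a short attack, set up for networked play.
; Inputs call Srv events that pass authority checks before Client events set axis, facing, dash and attack state.
; Tick turns that state into movement input, locking direction while dashing, and selects directional flipbooks and play rate.
; A helper zeroes velocity on unpushed axes to prevent wall gliding; SrvStopDashing is left unwired.
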(event Custom|srvStopDashing
  ;[1 1 1] Dash Handler
)

(event Custom|SrvUpdateDirection
  (params (Right :type Float%20%28single-precision%29) (Top :type Float%20%28single-precision%29))
  ;[1 1 1] Update Direction
  (Networking|SwitchHasAuthority
    (:Authority
      (CallFunction|ClientUpdateDirection Right Top))))

(event Custom|clientStopDashing
  ;[1 1 1] Dash Handler
  (Variables|Default|Setdashing? false))

(event Custom|ClientUpdateDirection
  (params (Right :type Float%20%28single-precision%29) (Top :type Float%20%28single-precision%29))
  ;[1 1 1] Update Direction
  (CallFunction|UpdateDirection Right Top)
  (if (or (!= Right 0.0) (!= Top 0.0))
    (Variables|Default|Setidle? false)
    (else
      (Variables|Default|Setidle? true))))

(event Custom|clientSetAttacking
  ;[1 1 1] Knight Attack
  (if (not (Variables|Default|Getattacking?))
    (Variables|Default|Setattacking? true)
    (Utilities|FlowControl|Delay 0.21)
    (Variables|Default|Setattacking? false)))

(event Custom|srvSetDashing
  ;[1 1 1] Dash Handler
  (Networking|SwitchHasAuthority
    (:Authority
      (CallFunction|ClientSetDashing))))

(event Custom|srvSetAttacking
  ;[1 1 1] Knight Attack
  (Networking|SwitchHasAuthority
    (:Authority
      (CallFunction|ClientSetAttacking))))

(event Custom|clientSetDashing
  ;[1 1 1] Dash Handler
  (if (not (or (Variables|Default|Getdashing?) (Variables|Default|Getidle?)))
    (Variables|Default|Setdashing? true)
    (Utilities|FlowControl|Delay (Variables|Default|GetDashPeriod))
    (Variables|Default|Setdashing? false)
    (Variables|Default|SetdashingVector "0, 0, 0")))

(event Custom|clientInputTop
  (params (NewParam :type Float%20%28single-precision%29))
  ;[1 1 1] Axis Input Handler
  (Variables|Default|SetaxisTop NewParam))

(event Custom|srvInputRight
  (params (NewParam :type Float%20%28single-precision%29))
  ;[1 1 1] Axis Input Handler
  (Networking|SwitchHasAuthority
    (:Authority
      (CallFunction|ClientInputRight NewParam))))

(event Custom|clientInputRight
  (params (NewParam :type Float%20%28single-precision%29))
  ;[1 1 1] Axis Input Handler
  (Variables|Default|SetaxisRight NewParam))

(event Custom|srvInputTop
  (params (NewParam :type Float%20%28single-precision%29))
  ;[1 1 1] Axis Input Handler
  (Networking|SwitchHasAuthority
    (:Authority
      (CallFunction|ClientInputTop NewParam))))

(event EventTick
  (params (DeltaSeconds :type Float%20%28single-precision%29))
  ;[1 1 1] Main Loop
  (Variables|Default|SetDeltaSeconds DeltaSeconds)
  (Utilities|FlowControl|Sequence
    (:then_0
      (CallFunction|ComputeDeltaMovement)
      (CallFunction|SrvUpdateDirection (Variables|Default|GetaxisRight) (Variables|Default|GetaxisTop)))
    (:then_1
      (CallFunction|UpdateAnimation)
      (if true
        (Pawn|Input|AddMovementInput (Variables|Default|GetDeltaMovement) 1.0 false)
        (CallFunction|PreventGlidingonWalls)))
    (:then_2
      (if (and (== (Variables|Default|GetaxisRight) 0.0) (== (Variables|Default|GetaxisTop) 0.0))
        (Variables|Default|Setidle? true)))))

(event Input|ActionEvents|InputActionAttack
  (params (Key :type Key%20Structure))
  ;[1 1 1] Knight Attack
  (:Pressed
    (CallFunction|SrvSetAttacking)))

(event Input|ActionEvents|InputActionDash
  (params (Key :type Key%20Structure))
  ;[1 1 1] Dash Handler
  (:Pressed
    (CallFunction|SrvSetDashing)))

(event Input|AxisEvents|InputAxisMoveRight
  (params (AxisValue :type Float%20%28single-precision%29))
  ;[1 1 1] Axis Input Handler
  (CallFunction|SrvInputRight AxisValue))

(event Input|AxisEvents|InputAxisMoveTop
  (params (AxisValue :type Float%20%28single-precision%29))
  ;[1 1 1] Axis Input Handler
  (CallFunction|SrvInputTop AxisValue))

(fn ConstructionScript
  (Variables|Default|SetMovementSpeed 1e+02)
  (Variables|Default|SetDashSpeedFactor 3.0)
  (Variables|Default|SetDashPeriod 0.5)
  (Variables|Default|SetableToDash? true))

(fn ComputeDeltaMovement
  (bind _axisright (Variables|Default|GetaxisRight))
  (bind _axistop (Variables|Default|GetaxisTop))
  (bind _returnvalue (* -1 _axistop))
  (bind _returnvalue_2 (Math|Vector|MakeVector _axisright _returnvalue 0.0))
  (bind _returnvalue_3 (Math|Vector|ClampVectorSize _returnvalue_2 0.0 1.0))
  (if (Variables|Default|Getdashing?)
    (if (Math|Vector|Equal(Vector) (Variables|Default|GetdashingVector) "0, 0, 0" 0.0001)
      (if (Math|Vector|Equal(Vector) _returnvalue_3 "0, 0, 0" 0.0001)
        (CallFunction|SrvStopDashing)
        (Variables|Default|SetDeltaMovement (* _returnvalue_3 (* (Variables|Default|GetDeltaSeconds) (Variables|Default|GetMovementSpeed))) :!label _label)
        (else
          (Variables|Default|SetdashingVector _returnvalue_3)
          (Variables|Default|SetDeltaMovement (* (Variables|Default|GetdashingVector) (* (Variables|Default|GetDashSpeedFactor) (* (Variables|Default|GetDeltaSeconds) (Variables|Default|GetMovementSpeed)))) :!label _label_2)))
      (else
        (goto _label_2)))
    (else
      (goto _label))))

(fn UpdateDirection
  (params (Right :type Float%20%28single-precision%29) (Top :type Float%20%28single-precision%29))
  (bind _returnvalue (> Right 0.0))
  (bind _returnvalue_2 (> Top 0.0))
  (bind _returnvalue_3 (< Top 0.0))
  (bind _returnvalue_4 (< Right 0.0))
  (bind _returnvalue_5 (== Right 0.0))
  (bind _returnvalue_6 (== Top 0.0))
  (if (and _returnvalue _returnvalue_6)
    (Variables|Default|SetLastMoveDirection "NewEnumerator0")
    (elif (and _returnvalue _returnvalue_2)
      (Variables|Default|SetLastMoveDirection "NewEnumerator1")
      (elif (and _returnvalue_2 _returnvalue_5)
        (Variables|Default|SetLastMoveDirection "NewEnumerator2")
        (elif (and _returnvalue_4 _returnvalue_2)
          (Variables|Default|SetLastMoveDirection "NewEnumerator3")
          (elif (and _returnvalue_4 _returnvalue_6)
            (Variables|Default|SetLastMoveDirection "NewEnumerator4")
            (elif (and _returnvalue_4 _returnvalue_3)
              (Variables|Default|SetLastMoveDirection "NewEnumerator5")
              (elif (and _returnvalue_5 _returnvalue_3)
                (Variables|Default|SetLastMoveDirection "NewEnumerator6")
                (elif (and _returnvalue _returnvalue_3)
                  (Variables|Default|SetLastMoveDirection "NewEnumerator7")
                  (elif (and _returnvalue_5 _returnvalue_6)
                    _))))))))))

(fn UpdateAnimation
  (if (Variables|Default|Getattacking?)
    (Sprite|SetFlipbook (Variables|Default|GetSprite) (Utilities|Select :Index (Variables|Default|GetLastMoveDirection) :NewEnumerator0 "/Game/Art/Flipbook/Kight_Attack/fb_RightAttackKnight.fb_RightAttackKnight" :NewEnumerator1 "/Game/Art/Flipbook/Kight_Attack/fb_TopRightAttackKnight.fb_TopRightAttackKnight" :NewEnumerator2 "/Game/Art/Flipbook/Kight_Attack/fb_TopAttackKnight.fb_TopAttackKnight" :NewEnumerator3 "/Game/Art/Flipbook/Kight_Attack/fb_TopLeftAttackKnight.fb_TopLeftAttackKnight" :NewEnumerator4 "/Game/Art/Flipbook/Kight_Attack/fb_LeftAttackKnight.fb_LeftAttackKnight" :NewEnumerator5 "/Game/Art/Flipbook/Kight_Attack/fb_BotLeftAttackKnight.fb_BotLeftAttackKnight" :NewEnumerator6 "/Game/Art/Flipbook/Kight_Attack/fb_BotAttackKnight.fb_BotAttackKnight" :NewEnumerator7 "/Game/Art/Flipbook/Kight_Attack/fb_BotRightAttackKinght.fb_BotRightAttackKinght"))
    (Components|Timeline|SetPlayRate (Variables|Default|GetSprite) 1.0)
    (else
      (Sprite|SetFlipbook (Variables|Default|GetSprite) (Utilities|Select :Index (Variables|Default|GetLastMoveDirection) :NewEnumerator0 "/Game/Art/Flipbook/Kight_Walk/fb_RightWalkKnight.fb_RightWalkKnight" :NewEnumerator1 "/Game/Art/Flipbook/Kight_Walk/fb_TopRighWalkKnight.fb_TopRighWalkKnight" :NewEnumerator2 "/Game/Art/Flipbook/Kight_Walk/fb_TopWalkKnight.fb_TopWalkKnight" :NewEnumerator3 "/Game/Art/Flipbook/Kight_Walk/fb_TopLeftWalkKnight.fb_TopLeftWalkKnight" :NewEnumerator4 "/Game/Art/Flipbook/Kight_Walk/fb_LeftWalkKnight.fb_LeftWalkKnight" :NewEnumerator5 "/Game/Art/Flipbook/Kight_Walk/fb_BotLeftWalkKnight.fb_BotLeftWalkKnight" :NewEnumerator6 "/Game/Art/Flipbook/Kight_Walk/fb_BotWalkKnight.fb_BotWalkKnight" :NewEnumerator7 "/Game/Art/Flipbook/Kight_Walk/fb_BotRightWalkKnight.fb_BotRightWalkKnight"))
      (if (Variables|Default|Getdashing?)
        (Components|Timeline|SetPlayRate (Variables|Default|GetSprite) 4.0)
        (elif (Variables|Default|Getidle?)
          (Components|Timeline|SetPlayRate (Variables|Default|GetSprite) 0.0)
          (else
            (Components|Timeline|SetPlayRate (Variables|Default|GetSprite) 1.0)))))))

(fn ParseInputs
  (bind _returnvalue (Input|AxisValues|GetMoveRight))
  (bind _returnvalue_2 (Input|AxisValues|GetMoveTop))
  (Utilities|FlowControl|Sequence
    (:then_0
      (if (not (== _returnvalue 0.0))
        (Variables|Default|SetaxisRight _returnvalue)
        (Variables|Default|SetmoveRightChange? false)))
    (:then_1
      (if (not (== _returnvalue_2 0.0))
        (Variables|Default|SetaxisTop _returnvalue_2)
        (Variables|Default|SetmoveTopChange? false)))))

(fn PreventGlidingonWalls
  (bind _deltamovement (Variables|Default|GetDeltaMovement))
  (bind _charactermovement (Variables|Character|GetCharacterMovement))
  (bind _returnvalue (Math|Vector|Normalize _deltamovement))
  (if (== (* (.x _returnvalue) (.x (Variables|/Script/Engine.MovementComponent|GetVelocity _charactermovement))) 0.0)
    (Variables|/Script/Engine.MovementComponent|SetVelocity _charactermovement (Math|Vector|MakeVector 0.0 (.y (Variables|/Script/Engine.MovementComponent|GetVelocity _charactermovement)) (.z (Variables|/Script/Engine.MovementComponent|GetVelocity _charactermovement)))))
  (if (== (* (.y _returnvalue) (.y (Variables|/Script/Engine.MovementComponent|GetVelocity _charactermovement))) 0.0)
    (Variables|/Script/Engine.MovementComponent|SetVelocity _charactermovement (Math|Vector|MakeVector (.x (Variables|/Script/Engine.MovementComponent|GetVelocity _charactermovement)) 0.0 (.z (Variables|/Script/Engine.MovementComponent|GetVelocity _charactermovement)))))
  (if (== (* (.z _returnvalue) (.z (Variables|/Script/Engine.MovementComponent|GetVelocity _charactermovement))) 0.0)
    (Variables|/Script/Engine.MovementComponent|SetVelocity _charactermovement (Math|Vector|MakeVector (.x (Variables|/Script/Engine.MovementComponent|GetVelocity _charactermovement)) (.y (Variables|/Script/Engine.MovementComponent|GetVelocity _charactermovement)) 0.0))))