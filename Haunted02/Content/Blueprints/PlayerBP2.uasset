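; Player Blueprint for a 2D knight that walks in eight directions on the XZ plane, dashes and attacks.
; Tick moves the actor with swept offsets, separately per axis when walking, then picks a walk or attack flipbook from the last input direction.
; Dash locks the input vector until a set distance is covered, with a Delay-based cooldown.
; Attack uses short Delays around a KnightAttack call, whose event here is empty.
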(event Custom|knightAttack
  ;[1 1 1] Knight Attack
)

(event EventTick
  (params (DeltaSeconds :type Float%20%28single-precision%29))
  ;[1 1 1] Main Loop
  (Utilities|FlowControl|Sequence
    (:then_0
      (CallFunction|MoveCharacter DeltaSeconds))
    (:then_1
      (CallFunction|SetMyFlipbook))))

(event Input|ActionEvents|InputActionAttack
  (params (Key :type Key%20Structure))
  ;[1 1 1] Knight Attack
  (:Pressed
    (if (not (Variables|Default|GetisAttacking))
      (Utilities|FlowControl|Sequence
        (:then_0
          (Variables|Default|SetisAttacking true)
          (Utilities|FlowControl|Delay 0.1)
          (CallFunction|KnightAttack))
        (:then_1
          (Utilities|FlowControl|Delay 0.15)
          (Variables|Default|SetisAttacking false))))))

(event Input|ActionEvents|InputActionDash
  (params (Key :type Key%20Structure))
  (bind _returnvalue (Input|AxisValues|GetMoveRight))
  (bind _returnvalue_2 (Input|AxisValues|GetMoveTop))
  (bind _returnvalue_3 (Math|Vector|MakeVector _returnvalue 0.0 _returnvalue_2))
  (bind _returnvalue_4 (Math|Vector|ClampVectorSize _returnvalue_3 0.0 1.0))
  ;[1 1 1] Dash Handler
  (:Pressed
    (if (not (or (Variables|Default|GetisDashing) (not (Variables|Default|GetisAbleToDash))))
      (if (!= (Math|Vector|VectorLength _returnvalue_4) 0.0)
        (Variables|Default|SetisDashing true)
        (Variables|Default|SetisAbleToDash false)
        (Variables|Default|SetdashingVector _returnvalue_4)
        (Utilities|FlowControl|Delay (Variables|Default|GetDashPeriod))
        (Variables|Default|SetisAbleToDash true)))))

(fn ConstructionScript
  (Variables|Default|SetMovementSpeed 1e+02)
  (Variables|Default|SetDashDistance 1e+02)
  (Variables|Default|SetDashSpeed 4e+02)
  (Variables|Default|SetDashPeriod 2.0)
  (Variables|Default|SetisAbleToDash true))

(fn SetMyFlipbook
  (bind _returnvalue (Input|AxisValues|GetMoveRight))
  (bind _returnvalue_2 (Input|AxisValues|GetMoveTop))
  (bind _returnvalue_3 (> _returnvalue 0.0))
  (bind _returnvalue_4 (> _returnvalue_2 0.0))
  (bind _returnvalue_5 (< _returnvalue_2 0.0))
  (bind _returnvalue_6 (< _returnvalue 0.0))
  (bind _returnvalue_7 (== _returnvalue 0.0))
  (bind _returnvalue_8 (== _returnvalue_2 0.0))
  ;[1 1 1] Direction Handler
  (if (and _returnvalue_3 _returnvalue_8)
    (Variables|Default|SetLastMoveDirection "NewEnumerator0")
    (elif (and _returnvalue_3 _returnvalue_4)
      (Variables|Default|SetLastMoveDirection "NewEnumerator1")
      (elif (and _returnvalue_4 _returnvalue_7)
        (Variables|Default|SetLastMoveDirection "NewEnumerator2")
        (elif (and _returnvalue_6 _returnvalue_4)
          (Variables|Default|SetLastMoveDirection "NewEnumerator3")
          (elif (and _returnvalue_6 _returnvalue_8)
            (Variables|Default|SetLastMoveDirection "NewEnumerator4")
            (elif (and _returnvalue_6 _returnvalue_5)
              (Variables|Default|SetLastMoveDirection "NewEnumerator5")
              (elif (and _returnvalue_7 _returnvalue_5)
                (Variables|Default|SetLastMoveDirection "NewEnumerator6")
                (elif (and _returnvalue_3 _returnvalue_5)
                  (Variables|Default|SetLastMoveDirection "NewEnumerator7")))))))))
  (if (Variables|Default|GetisAttacking)
    ;[1 1 1] Attack
    (Sprite|SetFlipbook (Variables|Default|GetSprite) (Utilities|Select :Index (Variables|Default|GetLastMoveDirection) :NewEnumerator0 "/Game/Art/Flipbook/Kight_Attack/fb_RightAttackKnight.fb_RightAttackKnight" :NewEnumerator1 "/Game/Art/Flipbook/Kight_Attack/fb_TopRightAttackKnight.fb_TopRightAttackKnight" :NewEnumerator2 "/Game/Art/Flipbook/Kight_Attack/fb_TopAttackKnight.fb_TopAttackKnight" :NewEnumerator3 "/Game/Art/Flipbook/Kight_Attack/fb_TopLeftAttackKnight.fb_TopLeftAttackKnight" :NewEnumerator4 "/Game/Art/Flipbook/Kight_Attack/fb_LeftAttackKnight.fb_LeftAttackKnight" :NewEnumerator5 "/Game/Art/Flipbook/Kight_Attack/fb_BotLeftAttackKnight.fb_BotLeftAttackKnight" :NewEnumerator6 "/Game/Art/Flipbook/Kight_Attack/fb_BotAttackKnight.fb_BotAttackKnight" :NewEnumerator7 "/Game/Art/Flipbook/Kight_Attack/fb_BotRightAttackKinght.fb_BotRightAttackKinght"))
    (Components|Timeline|SetPlayRate (Variables|Default|GetSprite) 1.0)
    (else
      ;[1 1 1] Walk
      (Sprite|SetFlipbook (Variables|Default|GetSprite) (Utilities|Select :Index (Variables|Default|GetLastMoveDirection) :NewEnumerator0 "/Game/Art/Flipbook/Kight_Walk/fb_RightWalkKnight.fb_RightWalkKnight" :NewEnumerator1 "/Game/Art/Flipbook/Kight_Walk/fb_TopRighWalkKnight.fb_TopRighWalkKnight" :NewEnumerator2 "/Game/Art/Flipbook/Kight_Walk/fb_TopWalkKnight.fb_TopWalkKnight" :NewEnumerator3 "/Game/Art/Flipbook/Kight_Walk/fb_TopLeftWalkKnight.fb_TopLeftWalkKnight" :NewEnumerator4 "/Game/Art/Flipbook/Kight_Walk/fb_LeftWalkKnight.fb_LeftWalkKnight" :NewEnumerator5 "/Game/Art/Flipbook/Kight_Walk/fb_BotLeftWalkKnight.fb_BotLeftWalkKnight" :NewEnumerator6 "/Game/Art/Flipbook/Kight_Walk/fb_BotWalkKnight.fb_BotWalkKnight" :NewEnumerator7 "/Game/Art/Flipbook/Kight_Walk/fb_BotRightWalkKnight.fb_BotRightWalkKnight"))
      (if (and _returnvalue_7 _returnvalue_8)
        (Components|Timeline|SetPlayRate (Variables|Default|GetSprite) 0.0)
        (elif (Variables|Default|GetisDashing)
          (Components|Timeline|SetPlayRate (Variables|Default|GetSprite) 4.0)
          (else
            (Components|Timeline|SetPlayRate (Variables|Default|GetSprite) 1.0))))))
  (return))

(fn MoveCharacter
  (params (deltaSeconds :type Float%20%28single-precision%29))
  (bind _returnvalue (Input|AxisValues|GetMoveRight))
  (bind _returnvalue_2 (Input|AxisValues|GetMoveTop))
  (bind _movementspeed (Variables|Default|GetMovementSpeed))
  (bind _movementspeed_2 (Variables|Default|GetMovementSpeed))
  (bind _dashspeed (Variables|Default|GetDashSpeed))
  (bind _dashingvector (Variables|Default|GetdashingVector))
  (bind _returnvalue_3 (Math|Vector|MakeVector _returnvalue 0.0 0.0))
  (bind _returnvalue_4 (Math|Vector|MakeVector 0.0 0.0 _returnvalue_2))
  (bind _returnvalue_5 (* deltaSeconds _movementspeed))
  (bind _returnvalue_6 (* deltaSeconds _movementspeed_2))
  (bind _returnvalue_7 (* deltaSeconds _dashspeed))
  (bind _returnvalue_8 (* _dashingvector _returnvalue_7))
  (bind _returnvalue_9 (Math|Vector|ClampVectorSize _returnvalue_3 0.0 1.0))
  (bind _returnvalue_10 (Math|Vector|ClampVectorSize _returnvalue_4 0.0 1.0))
  (bind _returnvalue_11 (* _returnvalue_10 _returnvalue_6))
  (bind _returnvalue_12 (* _returnvalue_9 _returnvalue_5))
  ;[1 1 1] Default Walking
  (if (Variables|Default|GetisDashing)
    ;[1 1 1] Dashing
    (if (>= (Variables|Default|GetcurrentDashDistance) (Variables|Default|GetDashDistance))
      (Variables|Default|SetcurrentDashDistance 0.0 :!label _label)
      (Variables|Default|SetisDashing false)
      (if (> (Math|Vector|VectorLength _returnvalue_12) 0.0) :!label _label_2
        (Transformation|AddActorWorldOffset _returnvalue_12 true))
      (if (> (Math|Vector|VectorLength _returnvalue_11) 0.0)
        (Transformation|AddActorWorldOffset _returnvalue_11 true))
      (else
        (Transformation|AddActorWorldOffset _returnvalue_8 true)
        (bind _output_get (Variables|Default|SetcurrentDashDistance (+ (Variables|Default|GetcurrentDashDistance) (Math|Vector|VectorLength _returnvalue_8))))
        (if (> _output_get (Variables|Default|GetDashDistance))
          (goto _label))))
    (else
      (goto _label_2))))